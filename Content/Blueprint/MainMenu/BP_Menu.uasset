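; BP_Menu is a main menu actor that shows the UI_MainMenu widget with a mouse cursor and drives an auto-aiming turret-like cube.
; A looping timer started on BeginPlay appears to drive TargetNearEnemie, which interpolates the cube's rotation toward the nearest BP_EnemieMenu within range.
; It then calls Fire, which line-traces along the cube's forward vector and sends GetHitMessage to the hit actor.
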(event `self.ReceiveBeginPlay`
  (bind _returnvalue (`GameplayStatics.GetPlayerController` 0))
  (set `PlayerController.bShowMouseCursor` true _returnvalue)
  (bind _returnvalue_2 (`|CreateWidget` "/Game/UI/UI_MainMenu.UI_MainMenu_C" _returnvalue))
  (`WidgetBlueprintLibrary.SetInputMode_UIOnlyEx` _returnvalue _returnvalue_2)
  (`UserWidget.AddToViewport` _returnvalue_2 0)
  (bind _returnvalue_3 (`KismetSystemLibrary.K2_SetTimerDelegate` (`|CreateDelegate` :!event `TargetNearEnemie`) 0.1 true))
  (set `self.MenuHandle` _returnvalue_3))

(event `TargetNearEnemie`
  (bind _outactors (`GameplayStatics.GetAllActorsOfClass` "/Game/Blueprint/MainMenu/BP_EnemieMenu.BP_EnemieMenu_C"))
  (bind (_distance _returnvalue) (`GameplayStatics.FindNearestActor` (`SceneComponent.K2_GetComponentLocation` (`self.Cube`)) _outactors))
  (if (< _distance 600.0)
    (`SceneComponent.K2_SetWorldRotation` (`self.Cube`) (`KismetMathLibrary.RInterpTo` (`SceneComponent.K2_GetComponentRotation` (`self.Cube`)) (`KismetMathLibrary.FindLookAtRotation` (`SceneComponent.K2_GetComponentLocation` (`self.Cube`)) (`self.K2_GetActorLocation` _returnvalue)) (`GameplayStatics.GetWorldDeltaSeconds`) 65.0) false false)
    (`self.Fire`)))

(event `Fire`
  (bind _cube (`self.Cube`))
  (bind _returnvalue (`SceneComponent.K2_GetComponentLocation` _cube))
  (bind _outhit (`KismetSystemLibrary.LineTraceSingleForObjects` :`Start` _returnvalue :`End` (+ _returnvalue (* (`SceneComponent.GetForwardVector` _cube) 700.0)) :`ObjectTypes` (`|MakeArray` "ObjectTypeQuery7" :!type "EObjectTypeQuery Enum") :`DrawTime` 2.5))
  (message `/Game/Blueprint/BPI_Shot.GetHit` (`.HitActor` (`GameplayStatics.BreakHitResult` _outhit))))

(fn `UserConstructionScript`)