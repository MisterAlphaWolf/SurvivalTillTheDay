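; Enemy Blueprint that can spawn a random weapon at its own location, based on a chance roll.
; RandomSpawnCondition sets SelectAWeapon when any of several random integer checks passes, and nothing in this graph resets the flag.
; When that flag is set, SpawnWeapon spawns a random class from WeaponToSpawn at the actor's location.
; Neither event is called within this graph.
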(event `RandomSpawnCondition`
  (bind _returnvalue (`KismetMathLibrary.RandomInteger` 10))
  (if (or (== _returnvalue 0) (== _returnvalue 2) (== _returnvalue 4) (== _returnvalue 6))
    (set `self.SelectAWeapon` true)))

(event `SpawnWeapon`
  (if (`self.SelectAWeapon`)
    (`|SpawnActorFromClass` (`KismetArrayLibrary.Array_Random` (`self.WeaponToSpawn`)) (`KismetMathLibrary.MakeTransform` (`self.K2_GetActorLocation`)) "Undefined" "MultiplyWithRoot" null null)))

(fn `UserConstructionScript`)