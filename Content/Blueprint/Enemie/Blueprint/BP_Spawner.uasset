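; BP_Spawner is an enemy spawner that populates waves using counters held in the GM_STTD game mode.
; StartWave starts a looping timer with a randomized start-delay variance.
; SpawnEnemie spawns a random class from EnemieClass at a random point inside its Box and decrements the remaining-to-spawn count until zero.
; EndWave clears the wave timer and calls the game mode's ResetTimer once NumberEnemieWave reaches zero.
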(event `StartWave`
  (bind _returnvalue (`KismetSystemLibrary.K2_SetTimerDelegate` (`|CreateDelegate` :!event `SpawnEnemie`) 0.5 true 0.0 (`KismetMathLibrary.RandomFloatInRange` 1.0 3.0)))
  (set `self.WaveManager` _returnvalue))

(event `SpawnEnemie`
  (bind _box (`self.Box`))
  (if (!= (`/Game/Blueprint/PlayerFoldier/GM_STTD.EnemieWaveToSpawn` (cast `/Game/Blueprint/PlayerFoldier/GM_STTD` (`GameplayStatics.GetGameMode`) :!pure true)) 0)
    (`|SpawnActorFromClass` (`KismetArrayLibrary.Array_Random` (`self.EnemieClass`)) (`KismetMathLibrary.MakeTransform` (`KismetMathLibrary.RandomPointInBoundingBox` (`SceneComponent.K2_GetComponentLocation` _box) (`BoxComponent.GetScaledBoxExtent` _box))) "AdjustIfPossibleButAlwaysSpawn" "MultiplyWithRoot" null null)
    (`/Engine/EditorBlueprintResources/StandardMacros.DecrementInt` (`/Game/Blueprint/PlayerFoldier/GM_STTD.EnemieWaveToSpawn` (cast `/Game/Blueprint/PlayerFoldier/GM_STTD` (`GameplayStatics.GetGameMode`) :!pure true)))))

(event `EndWave`
  (if (not (!= (`/Game/Blueprint/PlayerFoldier/GM_STTD.NumberEnemieWave` (cast `/Game/Blueprint/PlayerFoldier/GM_STTD` (`GameplayStatics.GetGameMode`) :!pure true)) 0))
    (`KismetSystemLibrary.K2_ClearAndInvalidateTimerHandle` (`self.WaveManager`))
    (`/Game/Blueprint/PlayerFoldier/GM_STTD.ResetTimer` (cast `/Game/Blueprint/PlayerFoldier/GM_STTD` (`GameplayStatics.GetGameMode`) :!pure true))))

(fn `UserConstructionScript`)