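; BP_EnemieRange is a ranged enemy with a blaster, counted by the game mode.
; A looping timer starts on BeginPlay, and a distance check fires when the player is within range.
; Firing is a debug-drawn Pawn line trace from the barrel socket, with its result unused.
; GetHit spawns a weapon, credits the player's kill, lowers the game mode's enemy count and destroys the actor.
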(event `/Game/Blueprint/BPI_Shot.GetHit`
  (`self.SpawnWeapon`)
  (`/Game/Blueprint/PlayerFoldier/BP_Player_Char.KillEnemie` (cast `/Game/Blueprint/PlayerFoldier/BP_Player_Char` (`GameplayStatics.GetPlayerCharacter` 0) :!pure true))
  (`/Game/Blueprint/PlayerFoldier/GM_STTD.ReduceNumberEnemie` (cast `/Game/Blueprint/PlayerFoldier/GM_STTD` (`GameplayStatics.GetGameMode`) :!pure true))
  (`self.K2_DestroyActor`))

(event `self.ReceiveBeginPlay`
  (`KismetSystemLibrary.K2_SetTimerDelegate` (`|CreateDelegate` :!event `CheckDistanceToPlayer`) 2.5 true))

(event `EnemiFire`
  (bind _blasterg (`self.blasterG`))
  (bind _returnvalue (`SceneComponent.GetSocketLocation` _blasterg "EndBarrel"))
  (`KismetSystemLibrary.LineTraceSingleForObjects` :`Start` _returnvalue :`End` (+ _returnvalue (* (`KismetMathLibrary.GetForwardVector` (`SceneComponent.GetSocketRotation` _blasterg "EndBarrel")) 500.0)) :`ObjectTypes` (`|MakeArray` "ObjectTypeQuery3" :!type "EObjectTypeQuery Enum") :`DrawDebugType` "ForDuration"))

(event `CheckDistanceToPlayer`
  (if (<= (`KismetMathLibrary.Vector_Distance` (`self.K2_GetActorLocation`) (`self.K2_GetActorLocation` (cast `/Game/Blueprint/PlayerFoldier/BP_Player_Char` (`GameplayStatics.GetPlayerCharacter` 0) :!pure true))) 500.0)
    (`self.EnemiFire`)))

(fn `UserConstructionScript`
  (`parent.UserConstructionScript`))