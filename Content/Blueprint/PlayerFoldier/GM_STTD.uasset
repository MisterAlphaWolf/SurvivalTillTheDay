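; GM_STTD, apparently a game mode, tracks wave state: a countdown, the enemy count and difficulty scaling.
; BeginPlay hides the cursor, sets game-only input and starts a looping one-second timer, presumably driving TimerWave, which counts down and clears the timer at zero.
; ReduceNumberEnemie decrements the enemy count, while WavePass scales it by DifficultyMultiplayer and truncates it.
; The Difficulty function maps EDifficulty to that multiplier but is not called here.
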(event Custom|ReduceNumberEnemie
  (Variables|Parametter|SetNumberEnemieWave (Math|Integer|Clamp(Integer) (- (Variables|Parametter|GetNumberEnemieWave) 1) 0 (Variables|Parametter|GetNumberEnemieWave))))

(event Custom|TimerWave
  (if (!= (Variables|Parametter|GetTimerWaveValue) 0)
    (Variables|Parametter|SetTimerWaveValue (Math|Integer|Clamp(Integer) (- (Variables|Parametter|GetTimerWaveValue) 1) 0 (Variables|Parametter|GetTimerWaveValue)))
    (else
      (Utilities|Time|ClearandInvalidateTimerbyHandle (Variables|Parametter|GetTimerHandle)))))

(event Custom|WavePass
  (Variables|Parametter|SetNumberEnemieWave (Math|Float|Truncate (|(A*B) (Variables|Parametter|GetNumberEnemieWave) (Variables|Parametter|GetDifficultyMultiplayer)))))

(event EventBeginPlay
  (bind _returnvalue (Game|GetPlayerController 0))
  (Variables|/Script/Engine.PlayerController|SetbShowMouseCursor _returnvalue false)
  (Input|SetInputModeGameOnly _returnvalue true)
  (bind _returnvalue_2 (Utilities|Time|SetTimerbyEvent (EventDispatchers|CreateEvent :!event Custom|TimerWave) 1.0 true))
  (Variables|Parametter|SetTimerHandle _returnvalue_2))

(fn ConstructionScript)

(fn Difficulty
  (switch Utilities|FlowControl|Switch|SwitchonE_Difficulty (Variables|Parametter|GetE_Difficulty)
    (:NewEnumerator0
      (Variables|Parametter|SetDifficultyMultiplayer 1.2))
    (:NewEnumerator1
      (Variables|Parametter|SetDifficultyMultiplayer 1.5))
    (:NewEnumerator2
      (Variables|Parametter|SetDifficultyMultiplayer 1.8)))
  (return))