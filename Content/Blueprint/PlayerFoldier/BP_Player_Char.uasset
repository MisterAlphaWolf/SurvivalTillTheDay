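; Player character for a shooter that moves relative to its rotatable mesh, counts kills as points and opens HUD, pause and death widgets.
; Weapon flags select automatic or semi-auto firing of short line traces from the barrel socket, with randomized yaw spread for shotguns, messaging hit actors.
; Dash teleports along a direction component, stopping at static-world impacts.
; Any hit taken pauses the game on the death screen.
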(event `self.ReceiveBeginPlay`
  (`EnhancedInputSubsystemInterface.AddMappingContext` (pcsubsystem `EnhancedInputLocalPlayerSubsystem` (`GameplayStatics.GetPlayerController` 0)) "/Game/Blueprint/PlayerFoldier/Input/IMC_STTD.IMC_STTD" 0 (struct))
  (bind _returnvalue (`|CreateWidget` "/Game/UI/UI_InGame.UI_InGame_C" (`GameplayStatics.GetPlayerController` 0)))
  (set `self.UI_Game` _returnvalue)
  (`UserWidget.AddToViewport` _returnvalue 0))

(event `EnhancedInput|/Game/Blueprint/PlayerFoldier/Input/InputAction/IA_MoveLeftAndRight`
  (params (ActionValue :type "Float (double-precision)") (ElapsedSeconds :type "Float (double-precision)") (TriggeredSeconds :type "Float (double-precision)") (InputAction :type "InputAction Object Reference" :default "/Game/Blueprint/PlayerFoldier/Input/InputAction/IA_MoveLeftAndRight.IA_MoveLeftAndRight"))
  (:`Triggered`
    (`self.AddMovementInput` (`SceneComponent.GetForwardVector` (`self.Mesh`)) ActionValue)))

(event `EnhancedInput|/Game/Blueprint/PlayerFoldier/Input/InputAction/IA_MoveUpAndDown`
  (params (ActionValue :type "Float (double-precision)") (ElapsedSeconds :type "Float (double-precision)") (TriggeredSeconds :type "Float (double-precision)") (InputAction :type "InputAction Object Reference" :default "/Game/Blueprint/PlayerFoldier/Input/InputAction/IA_MoveUpAndDown.IA_MoveUpAndDown"))
  (:`Triggered`
    (`self.AddMovementInput` (`SceneComponent.GetRightVector` (`self.Mesh`)) ActionValue)))

(event `EnhancedInput|/Game/Blueprint/PlayerFoldier/Input/InputAction/IA_RotateLeftAndRight`
  (params (ActionValue :type "Float (double-precision)") (ElapsedSeconds :type "Float (double-precision)") (TriggeredSeconds :type "Float (double-precision)") (InputAction :type "InputAction Object Reference" :default "/Game/Blueprint/PlayerFoldier/Input/InputAction/IA_RotateLeftAndRight.IA_RotateLeftAndRight"))
  (bind _mesh (`self.Mesh`))
  (:`Triggered`
    (`SceneComponent.K2_SetWorldRotation` _mesh (`KismetMathLibrary.MakeRotator` (.roll (`SceneComponent.K2_GetComponentRotation` _mesh)) (.pitch (`SceneComponent.K2_GetComponentRotation` _mesh)) (+ (.yaw (`SceneComponent.K2_GetComponentRotation` _mesh)) ActionValue)) false false)))

(event `EnhancedInput|/Game/Blueprint/PlayerFoldier/Input/InputAction/IA_Fire`
  (params (ActionValue :type Boolean) (ElapsedSeconds :type "Float (double-precision)") (TriggeredSeconds :type "Float (double-precision)") (InputAction :type "InputAction Object Reference" :default "/Game/Blueprint/PlayerFoldier/Input/InputAction/IA_Fire.IA_Fire"))
  (bind _array (`|MakeArray` "ObjectTypeQuery7" :!type "EObjectTypeQuery Enum"))
  (bind _blasterb (`self.blasterB`))
  (bind _blasterb_2 (`self.blasterB`))
  (bind _returnvalue (`SceneComponent.GetSocketLocation` _blasterb_2 "EndBarrel"))
  (bind _returnvalue_2 (`SceneComponent.GetSocketLocation` _blasterb "EndBarrel"))
  (:`Triggered`
    (if (`self.AutoWeapon`)
      (if (`self.ShotGunWeapon`) :!label _label
        (for _ (range 16)
          (bind _outhit (`KismetSystemLibrary.LineTraceSingleForObjects` _returnvalue (+ _returnvalue (* (`KismetMathLibrary.GreaterGreater_VectorRotator` (`KismetMathLibrary.GetForwardVector` (`SceneComponent.GetSocketRotation` _blasterb_2 "EndBarrel")) (`KismetMathLibrary.MakeRotator` 0.0 0.0 (`KismetMathLibrary.RandomFloatInRange` -25.0 25.0))) 700.0)) _array))
          (message `/Game/Blueprint/BPI_Shot.GetHit` (`.HitActor` (`GameplayStatics.BreakHitResult` _outhit))))
        (else
          (bind _outhit_2 (`KismetSystemLibrary.LineTraceSingleForObjects` _returnvalue_2 (+ _returnvalue_2 (* (`KismetMathLibrary.GetForwardVector` (`SceneComponent.GetSocketRotation` _blasterb "EndBarrel")) 700.0)) _array))
          (message `/Game/Blueprint/BPI_Shot.GetHit` (`.HitActor` (`GameplayStatics.BreakHitResult` _outhit_2)))))))
  (:`Started`
    (if (`self.SemiWeapon`)
      (goto _label))))

(event `/Game/Blueprint/BPI_Shot.GetHit`
  (bind _returnvalue (`GameplayStatics.GetPlayerController` 0))
  (`GameplayStatics.SetGamePaused` true)
  (bind _returnvalue_2 (`|CreateWidget` "/Game/UI/UI_Death.UI_Death_C" _returnvalue))
  (`WidgetBlueprintLibrary.SetInputMode_UIOnlyEx` _returnvalue _returnvalue_2)
  (`UserWidget.AddToViewport` _returnvalue_2 0))

(event `KillEnemie`
  (`/Engine/EditorBlueprintResources/StandardMacros.IncrementInt` (`self.Point`)))

(event `EnhancedInput|/Game/Blueprint/PlayerFoldier/Input/InputAction/IA_Pause`
  (params (ActionValue :type Boolean) (ElapsedSeconds :type "Float (double-precision)") (TriggeredSeconds :type "Float (double-precision)") (InputAction :type "InputAction Object Reference" :default "/Game/Blueprint/PlayerFoldier/Input/InputAction/IA_Pause.IA_Pause"))
  (bind _returnvalue (`GameplayStatics.GetPlayerController` 0))
  (:`Started`
    (bind _returnvalue_2 (`|CreateWidget` "/Game/UI/UI_Pause.UI_Pause_C" (`GameplayStatics.GetPlayerController` 0)))
    (set `self.PauseMenu` _returnvalue_2)
    (`UserWidget.AddToViewport` _returnvalue_2 0)
    (`WidgetBlueprintLibrary.SetInputMode_UIOnlyEx` _returnvalue (`self.PauseMenu`))
    (set `PlayerController.bShowMouseCursor` true _returnvalue)
    (`GameplayStatics.SetGamePaused` true)))

(event `EnhancedInput|/Game/Blueprint/PlayerFoldier/Input/InputAction/IA_Dash`
  (params (ActionValue :type Boolean) (ElapsedSeconds :type "Float (double-precision)") (TriggeredSeconds :type "Float (double-precision)") (InputAction :type "InputAction Object Reference" :default "/Game/Blueprint/PlayerFoldier/Input/InputAction/IA_Dash.IA_Dash"))
  (bind _directionofdash (`self.DirectionOfDash`))
  (bind _returnvalue (`SceneComponent.K2_GetComponentLocation` _directionofdash))
  (:`Started`
    (bind (_outhit _returnvalue_2) (`KismetSystemLibrary.LineTraceSingleForObjects` _returnvalue (+ _returnvalue (* (`KismetMathLibrary.GetForwardVector` (`SceneComponent.K2_GetComponentRotation` _directionofdash)) 400.0)) (`|MakeArray` "ObjectTypeQuery1" :!type "EObjectTypeQuery Enum")))
    (if _returnvalue_2
      (bind (_bblockinghit _binitialoverlap _time _distance _location _impactpoint _normal _impactnormal _physmat _hitactor _hitcomponent _hitbonename _bonename _hititem _elementindex _faceindex _tracestart _traceend) (`GameplayStatics.BreakHitResult` _outhit))
      (`self.K2_TeleportTo` _impactpoint (`SceneComponent.K2_GetComponentRotation` (`self.Mesh`)))
      (else
        (`self.K2_TeleportTo` _traceend (`SceneComponent.K2_GetComponentRotation` (`self.Mesh`)))))))

(event `ChangeMesh`
  (params (NewWeaponMesh :type "StaticMesh Object Reference"))
  (`StaticMeshComponent.SetStaticMesh` (`self.blasterB`) NewWeaponMesh))

(fn `UserConstructionScript`)