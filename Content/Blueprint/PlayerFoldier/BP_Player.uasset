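; BP_Player is the player pawn, moved and yawed through Enhanced Input using the IMC_STTD mapping context added on BeginPlay.
; Movement follows the Cube component's forward and right vectors, and rotation input adds to that Cube's world yaw.
; Firing alternates via FlipFlop between right and left guns, spawning BP_Bullet at each EndBarrel socket.
; KillEnemie increments the Point score and prints it.
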(event `self.ReceiveBeginPlay`
  (`EnhancedInputSubsystemInterface.AddMappingContext` (pcsubsystem `EnhancedInputLocalPlayerSubsystem` (`GameplayStatics.GetPlayerController` 0)) "/Game/Blueprint/PlayerFoldier/Input/IMC_STTD.IMC_STTD" 0 (struct)))

(event `EnhancedInput|/Game/Blueprint/PlayerFoldier/Input/InputAction/IA_MoveLeftAndRight`
  (params (ActionValue :type "Float (double-precision)") (ElapsedSeconds :type "Float (double-precision)") (TriggeredSeconds :type "Float (double-precision)") (InputAction :type "InputAction Object Reference" :default "/Game/Blueprint/PlayerFoldier/Input/InputAction/IA_MoveLeftAndRight.IA_MoveLeftAndRight"))
  (:`Triggered`
    (`self.AddMovementInput` (`SceneComponent.GetRightVector` (`self.Cube`)) ActionValue)))

(event `EnhancedInput|/Game/Blueprint/PlayerFoldier/Input/InputAction/IA_MoveUpAndDown`
  (params (ActionValue :type "Float (double-precision)") (ElapsedSeconds :type "Float (double-precision)") (TriggeredSeconds :type "Float (double-precision)") (InputAction :type "InputAction Object Reference" :default "/Game/Blueprint/PlayerFoldier/Input/InputAction/IA_MoveUpAndDown.IA_MoveUpAndDown"))
  (:`Triggered`
    (`self.AddMovementInput` (`SceneComponent.GetForwardVector` (`self.Cube`)) ActionValue)))

(event `EnhancedInput|/Game/Blueprint/PlayerFoldier/Input/InputAction/IA_RotateLeftAndRight`
  (params (ActionValue :type "Float (double-precision)") (ElapsedSeconds :type "Float (double-precision)") (TriggeredSeconds :type "Float (double-precision)") (InputAction :type "InputAction Object Reference" :default "/Game/Blueprint/PlayerFoldier/Input/InputAction/IA_RotateLeftAndRight.IA_RotateLeftAndRight"))
  (bind _cube (`self.Cube`))
  (:`Triggered`
    (`SceneComponent.K2_SetWorldRotation` _cube (`KismetMathLibrary.MakeRotator` (.roll (`SceneComponent.K2_GetComponentRotation` _cube)) (.pitch (`SceneComponent.K2_GetComponentRotation` _cube)) (+ (.yaw (`SceneComponent.K2_GetComponentRotation` _cube)) ActionValue)) false false)))

(event `EnhancedInput|/Game/Blueprint/PlayerFoldier/Input/InputAction/IA_Fire`
  (params (ActionValue :type Boolean) (ElapsedSeconds :type "Float (double-precision)") (TriggeredSeconds :type "Float (double-precision)") (InputAction :type "InputAction Object Reference" :default "/Game/Blueprint/PlayerFoldier/Input/InputAction/IA_Fire.IA_Fire"))
  (bind _gunmeshright (`self.GunMeshRight`))
  (bind _gunmeshleft (`self.GunMeshLeft`))
  (:`Started`
    (`/Engine/EditorBlueprintResources/StandardMacros.FlipFlop`
      (:`A`
        (`|SpawnActorFromClass` "/Game/Blueprint/PlayerFoldier/BP_Bullet.BP_Bullet_C" (`KismetMathLibrary.MakeTransform` (`SceneComponent.GetSocketLocation` _gunmeshright "EndBarrel") (`SceneComponent.GetSocketRotation` _gunmeshright "EndBarrel")) "Undefined" "MultiplyWithRoot" null null))
      (:`B`
        (`|SpawnActorFromClass` "/Game/Blueprint/PlayerFoldier/BP_Bullet.BP_Bullet_C" (`KismetMathLibrary.MakeTransform` (`SceneComponent.GetSocketLocation` _gunmeshleft "EndBarrel") (`SceneComponent.GetSocketRotation` _gunmeshleft "EndBarrel")) "Undefined" "MultiplyWithRoot" null null)))))

(event `KillEnemie`
  (bind _result (`/Engine/EditorBlueprintResources/StandardMacros.IncrementInt` (`self.Point`))
    (:`  `
      (`KismetSystemLibrary.PrintString` (`KismetStringLibrary.Concat_StrStr` "Player Point : " (`KismetStringLibrary.Conv_IntToString` _result))))))

(fn `UserConstructionScript`)